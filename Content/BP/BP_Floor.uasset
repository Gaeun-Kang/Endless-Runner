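; BP_Floor is a floor tile for an endless-runner style game that chains new tiles as the player advances.
; Construction gathers three trap-point transforms and adds a child actor at a randomly chosen one.
; When BP_ThirdPersonCharacter overlaps the Box, it asks BP_EndlessGamemode to add a tile, then destroys itself two seconds later.
; GetAttachTransform exposes the Arrow's world transform as an attach point.
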(event `self.Box.OnComponentBeginOverlap`
  (params (OverlappedComponent :type "PrimitiveComponent Object Reference") (OtherActor :type "Actor Object Reference") (OtherComp :type "PrimitiveComponent Object Reference") (OtherBodyIndex :type Integer) (bFromSweep :type Boolean) (SweepResult :type "HitResult Structure (by ref)"))
  (cast `/Game/ThirdPerson/Blueprints/BP_ThirdPersonCharacter` OtherActor)
  (bind _asbp_endless_gamemode (cast `/Game/ThirdPerson/Blueprints/BP_EndlessGamemode` (`GameplayStatics.GetGameMode`)))
  (`/Game/ThirdPerson/Blueprints/BP_EndlessGamemode.AddFloorTile` _asbp_endless_gamemode)
  (`KismetSystemLibrary.Delay` 2.0)
  (`self.K2_DestroyActor`))

(fn `GetAttachTransform`
  (returns (AttachTransform :type "Transform Structure"))
  (return (`SceneComponent.K2_GetComponentToWorld` (`self.Arrow`))))

(fn `Set Spawn Points`
  (for _ (range 3)
    (set `self.SpawnTransform` (`|MakeArray` (`SceneComponent.GetRelativeTransform` (`self.SpawnTrap`)) (`SceneComponent.GetRelativeTransform` (`self.SpawnTrapL`)) (`SceneComponent.GetRelativeTransform` (`self.SpawnTrapR`))))))

(fn `SpawnTraper`
  (bind _spawntransform (`self.SpawnTransform`))
  (`AddComponent|NODE_AddChildActorComponent-0` :`RelativeTransform` (`|GetArrayItem` _spawntransform (`KismetMathLibrary.RandomIntegerInRange` 0 (`KismetArrayLibrary.Array_LastIndex` _spawntransform)))))

(fn `UserConstructionScript`
  (`self.Set Spawn Points`)
  (`self.SpawnTraper`))